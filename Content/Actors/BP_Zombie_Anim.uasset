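; Side-scroller zombie enemy character that patrols back and forth and kills the player on contact unless they are in zombie form.
; It walks forward every tick, flipping yaw through TurnChar at walls, floor edges and overlapping capsule hits.
; AI perception raises its speed with a growl when it senses a living, non-zombie player, and slows it when that player is lost or dead.
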(event `self.ReceiveTick`
  (params (DeltaSeconds :type "Float (single-precision)"))
  ;[0.1387 0.1437 0.15 0.5] Move Forward
  (`self.AddMovementInput` (`self.GetActorForwardVector`) (`self.SpeedScale`)))

(event `self.Wall Detector.OnComponentBeginOverlap`
  (params (OverlappedComponent :type "PrimitiveComponent Object Reference") (OtherActor :type "Actor Object Reference") (OtherComp :type "PrimitiveComponent Object Reference") (OtherBodyIndex :type Integer) (bFromSweep :type Boolean) (SweepResult :type "HitResult Structure (by ref)"))
  ;[0.09655 0.1163 0.15 0.5] Turn Around at Walls
  (`self.TurnChar`))

(event `self.FloorDetector.OnComponentEndOverlap`
  (params (OverlappedComponent :type "PrimitiveComponent Object Reference") (OtherActor :type "Actor Object Reference") (OtherComp :type "PrimitiveComponent Object Reference") (OtherBodyIndex :type Integer))
  ;[0.1206 0.15 0.1377 0.5] Turn Around at Cliffs
  (if (not (> (`KismetArrayLibrary.Array_Length` (`PrimitiveComponent.GetOverlappingActors` (`self.FloorDetector`) "/Script/Engine.StaticMeshActor")) 0))
    (`self.TurnChar`)))

(event `self.PlayerAttack.OnComponentBeginOverlap`
  (params (OverlappedComponent :type "PrimitiveComponent Object Reference") (OtherActor :type "Actor Object Reference") (OtherComp :type "PrimitiveComponent Object Reference") (OtherBodyIndex :type Integer) (bFromSweep :type Boolean) (SweepResult :type "HitResult Structure (by ref)"))
  ;[0.15 0.09604 0.08856 0.5] Damage Player
  (bind _asside_scroller_character (cast `/Game/SideScrollerBP/Blueprints/SideScrollerCharacter` OtherActor))
  (if (not (`/Game/SideScrollerBP/Blueprints/SideScrollerCharacter.IsInZombieForm` _asside_scroller_character))
    (`/Game/SideScrollerBP/Blueprints/SideScrollerCharacter.Death` _asside_scroller_character)))

(event `self.AIPerception.OnTargetPerceptionUpdated`
  (params (Actor :type "Actor Object Reference") (Stimulus :type "AIStimulus Structure"))
  ;[0.1303 0.15 0.1046 0.5] Detect Player
  (bind _asside_scroller_character (cast `/Game/SideScrollerBP/Blueprints/SideScrollerCharacter` Actor))
  (if (`/Game/SideScrollerBP/Blueprints/SideScrollerCharacter.IsAlive` _asside_scroller_character)
    (if (`/Game/SideScrollerBP/Blueprints/SideScrollerCharacter.IsInZombieForm` _asside_scroller_character)
      _
      (elif (`.bSuccessfullySensed` (break `AIStimulus` Stimulus))
        (`GameplayStatics.PlaySound2D` "/Game/Audio/WAV_Zombie_Rahh.WAV_Zombie_Rahh" 0.55 0.85 0.0 null null)
        (set `self.SpeedScale` 1.0)
        (else
          (set `self.SpeedScale` 0.3 :!label _label))))
    (else
      (goto _label))))

(event `self.CapsuleComponent.OnComponentHit`
  (params (HitComponent :type "PrimitiveComponent Object Reference") (OtherActor :type "Actor Object Reference") (OtherComp :type "PrimitiveComponent Object Reference") (NormalImpulse :type "Vector Structure") (Hit :type "HitResult Structure (by ref)"))
  (if (`PrimitiveComponent.IsOverlappingActor` (`self.CapsuleComponent`) OtherActor)
    (`KismetSystemLibrary.Delay` 0.2)
    (`self.TurnChar`)))

(fn `TurnChar`
  (bind (_returnvalue_roll _returnvalue_pitch _returnvalue_yaw) (`KismetMathLibrary.BreakRotator` (`self.K2_GetActorRotation`)))
  (if (> _returnvalue_yaw 0.0)
    (`self.K2_SetActorRotation` (`KismetMathLibrary.MakeRotator` _returnvalue_roll _returnvalue_pitch -90.0))
    (else
      (`self.K2_SetActorRotation` (`KismetMathLibrary.MakeRotator` _returnvalue_roll _returnvalue_pitch 90.0)))))

(fn `UserConstructionScript`)